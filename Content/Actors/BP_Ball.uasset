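; BP_Ball is the physics-driven ball of a brick-breaker game, launched along negative X on BeginPlay.
; Overlaps with bricks, walls and the paddle play a sound, and bricks also spawn a destruction particle.
; Brick and wall hits raise BallSpeed, then clamp velocity to exactly that magnitude, keeping its direction.
; Touching BP_WallEnd destroys the ball, decrements the paddle's ball count and, at zero, disables input and shows the replay menu.
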(event `self.ReceiveBeginPlay`
  (`PrimitiveComponent.SetPhysicsLinearVelocity` (`self.Sphere`) (-1200.0 0.0 0.0) false "None"))

(event `self.ReceiveActorBeginOverlap`
  (params (OtherActor :type "Actor Object Reference"))
  (bind _ballspeed (`self.ballSpeed`))
  (bind _asbp_brick (cast `/Game/Actors/BP_Brick` OtherActor)
    (:`then`
      (bind _returnvalue (`self.K2_GetActorLocation` _asbp_brick))
      (`GameplayStatics.SpawnSoundAtLocation` "/Game/Sounds/BallSound.BallSound" _returnvalue (struct) 1.0 1.0 0.0 null null)
      (`GameplayStatics.SpawnEmitterAtLocation` "/Game/Realistic_Starter_VFX_Pack_Vol2/Particles/Destruction/P_Destruction_Wood.P_Destruction_Wood" _returnvalue)
      (set `self.ballSpeed` (+ (`self.ballSpeed`) 10) :!label _label)
      (bind _returnvalue_2 (`PrimitiveComponent.GetPhysicsLinearVelocity` (`self.Sphere`) "None"))
      (`PrimitiveComponent.SetPhysicsLinearVelocity` (`self.Sphere`) (`KismetMathLibrary.ClampVectorSize` _returnvalue_2 _ballspeed _ballspeed) false "None"))
    (:`CastFailed`
      (cast `/Game/Actors/BP_Wall` OtherActor
        (:`then`
          (`GameplayStatics.SpawnSoundAtLocation` "/Game/Sounds/BallSound.BallSound" (`self.K2_GetActorLocation`) (struct) 1.0 1.0 0.0 null null)
          (goto _label))
        (:`CastFailed`
          (cast `/Game/Actors/BP_WallEnd` OtherActor
            (:`then`
              (`self.K2_DestroyActor`)
              (bind _asbp_paddle (cast `/Game/Actors/BP_Paddle` (`GameplayStatics.GetPlayerPawn` 0)))
              (bind _output_get (set `/Game/Actors/BP_Paddle.nbBall` (- (`/Game/Actors/BP_Paddle.nbBall` _asbp_paddle) 1) _asbp_paddle))
              (if (== _output_get 0)
                (bind _returnvalue_3 (`|CreateWidget` "/Game/Widgets/Replay_Menu.Replay_Menu_C"))
                (`self.DisableInput` (`GameplayStatics.GetPlayerPawn` 0) null)
                (`UserWidget.AddToViewport` _returnvalue_3 0)
                (set `PlayerController.bShowMouseCursor` true (`GameplayStatics.GetPlayerController` 0))))
            (:`CastFailed`
              (cast `/Game/Actors/BP_Paddle` OtherActor)
              (`GameplayStatics.SpawnSoundAtLocation` "/Game/Sounds/BallSound.BallSound" (`self.K2_GetActorLocation`) (struct) 1.0 1.0 0.0 null null))))))))

(fn `UserConstructionScript`)