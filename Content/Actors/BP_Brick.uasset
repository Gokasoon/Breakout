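; BP_Brick is a breakout-style brick that loses HP when a BP_Ball overlaps it and awards score to the player's BP_Paddle.
; BeginPlay randomly sets HP and matching color, weighted toward the toughest red, or occasionally makes a one-hit green bonus brick.
; Each hit recolors the brick, and the last destroys it with explosion effect and sound.
; Bonus bricks also spawn an extra ball and raise the paddle's ball count.
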(event `self.ReceiveActorBeginOverlap`
  (params (OtherActor :type "Actor Object Reference"))
  (bind _hp (`self.HP`))
  (cast `/Game/Actors/BP_Ball` OtherActor)
  (if (== _hp 1)
    (bind _asbp_paddle (cast `/Game/Actors/BP_Paddle` (`GameplayStatics.GetPlayerPawn` 0)))
    (set `/Game/Actors/BP_Paddle.score` (+ (`/Game/Actors/BP_Paddle.score` _asbp_paddle) 5) _asbp_paddle)
    (`self.K2_DestroyActor`)
    (`GameplayStatics.SpawnEmitterAtLocation` "/Game/StarterContent/Particles/P_Explosion.P_Explosion" (`self.K2_GetActorLocation`))
    (`GameplayStatics.PlaySound2D` "/Game/StarterContent/Audio/Explosion01.Explosion01" 1.0 1.0 0.0 null null)
    (if (== true (`self.Bonus`))
      (bind _asbp_paddle_2 (cast `/Game/Actors/BP_Paddle` (`GameplayStatics.GetPlayerPawn` 0)))
      (set `/Game/Actors/BP_Paddle.nbBall` (+ (`/Game/Actors/BP_Paddle.nbBall` _asbp_paddle_2) 1) _asbp_paddle_2)
      (bind _returnvalue (`|SpawnActorFromClass` "/Game/Actors/BP_Ball.BP_Ball_C" (`KismetMathLibrary.Conv_VectorToTransform` (`self.K2_GetActorLocation`)) "Undefined" "MultiplyWithRoot" null null))
      (bind _sphere1 (`/Game/Actors/BP_Ball.Sphere1` _returnvalue))
      (bind _returnvalue_2 (`PrimitiveComponent.GetPhysicsLinearVelocity` _sphere1 "None"))
      (`PrimitiveComponent.SetPhysicsLinearVelocity` _sphere1 (`KismetMathLibrary.MakeVector` (.x _returnvalue_2) -1200.0 (.z _returnvalue_2)) false "None"))
    (elif (== 2 _hp)
      (set `self.HP` 1)
      (`PrimitiveComponent.SetMaterial` (`self.Cube`) 0 "/Game/Materials/Yellow.Yellow")
      (bind _asbp_paddle_3 (cast `/Game/Actors/BP_Paddle` (`GameplayStatics.GetPlayerPawn` 0)))
      (set `/Game/Actors/BP_Paddle.score` (+ (`/Game/Actors/BP_Paddle.score` _asbp_paddle_3) 1) _asbp_paddle_3)
      (elif (== _hp 3)
        (set `self.HP` 2)
        (`PrimitiveComponent.SetMaterial` (`self.Cube`) 0 "/Game/Materials/Orange.Orange")
        (bind _asbp_paddle_4 (cast `/Game/Actors/BP_Paddle` (`GameplayStatics.GetPlayerPawn` 0)))
        (set `/Game/Actors/BP_Paddle.score` (+ (`/Game/Actors/BP_Paddle.score` _asbp_paddle_4) 1) _asbp_paddle_4)))))

(event `self.ReceiveBeginPlay`
  (bind _hp (`self.HP`))
  (if (== 1 (`KismetMathLibrary.RandomInteger` 15))
    (set `self.Bonus` true)
    (`PrimitiveComponent.SetMaterial` (`self.Cube`) 0 "/Game/Materials/Green.Green")
    (set `self.HP` 1)
    (else
      (set `self.HP` (`KismetMathLibrary.RandomInteger` 4))
      (if (== _hp 1)
        (`PrimitiveComponent.SetMaterial` (`self.Cube`) 0 "/Game/Materials/Yellow.Yellow")
        (elif (== _hp 2)
          (`PrimitiveComponent.SetMaterial` (`self.Cube`) 0 "/Game/Materials/Orange.Orange")
          (elif (== 3 _hp)
            (`PrimitiveComponent.SetMaterial` (`self.Cube`) 0 "/Game/Materials/Red.Red" :!label _label)
            (elif (== _hp 0)
              (set `self.HP` 3)
              (goto _label))))))))

(fn `UserConstructionScript`)